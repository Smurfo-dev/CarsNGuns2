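; Base player controller Blueprint that adds two debug-style hotkeys, both routed through managers on the DefaultGameState.
; P gets the missions from the mission manager and prints each one's info under an on-screen "Mission Log" header.
; H asks the enemy manager to spawn a BP_SportsHeavyEnemy, passing this controller.
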(event EventBeginPlay)

(event EventTick
  (params (DeltaSeconds :type Float%20%28single-precision%29)))

(event Input|KeyboardEvents|H
  (params (Key :type Key%20Structure :default "None"))
  (:Pressed
    (bind _asdefault_game_state (Utilities|Casting|CastToDefaultGameState (Game|GetGameState)))
    (Class|EnemyManager|SpawnEnemy (Class|DefaultGameState|GetEnemyManager _asdefault_game_state) self "/Game/Blueprints/Enemies/Vehicles/BP_SportsHeavyEnemy.BP_SportsHeavyEnemy_C")))

(event Input|KeyboardEvents|P
  (params (Key :type Key%20Structure :default "None"))
  (:Pressed
    (bind _asdefault_game_state (Utilities|Casting|CastToDefaultGameState (Game|GetGameState)))
    (bind _returnvalue (Class|MissionManager|GetMissions (Class|DefaultGameState|GetMissionManager _asdefault_game_state)))
    (Development|PrintString "Mission Log: " true false "(R=0.107261,G=1.000000,B=0.493208,A=1.000000)")
    (for _array_element _returnvalue
      (Class|BaseMission|PrintMissionInfo _array_element))
    (Development|PrintString "Mission Log Printed" false)))

(fn ConstructionScript)